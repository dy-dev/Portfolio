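; Actor that imports 3D model files from disk through AssimpImporter and displays them as procedural meshes.
; CreateNewMesh runs at BeginPlay and from the Construction Script (hard-coded test OBJ), replacing the previous mesh.
; It inverts normals, applies the importer's material, and falls back to the importer's internal path when loading fails.
; ApplyTexture similarly builds a mesh from that internal path, without removing the previous one.
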(event `self.ReceiveBeginPlay`
  (`self.CreateNewMesh` (`self.FilePath`)))

(event `self.ReceiveActorBeginOverlap`
  (params (OtherActor :type "Actor Object Reference")))

(event `self.ReceiveTick`
  (params (DeltaSeconds :type "Float (single-precision)")))

(fn `ApplyTexture`
  (bind _assimpimporter (`self.AssimpImporter`))
  (bind _assimpimporter_2 (`self.AssimpImporter`))
  (bind _internalfilepath (`AssimpImporterComponent.InternalFilePath` _assimpimporter))
  (set `self.FilePath` _internalfilepath)
  (set `AssimpImporterComponent.InverseNormals` true _assimpimporter)
  (bind _returnvalue (`AssimpImporterComponent.Load3DModel` _assimpimporter (`self.FilePath`)))
  (if _returnvalue
    (bind _returnvalue_2 (`AddComponent|ProceduralMeshComponent_1`))
    (`AssimpImporterComponent.SetMaterialToProceduralMeshComp` _assimpimporter_2 _returnvalue_2)
    (`ProceduralMeshComponent.CreateMeshSection` :`self` _returnvalue_2 :`Vertices` (`AssimpImporterComponent.Vertices` _assimpimporter_2) :`Triangles` (`AssimpImporterComponent.Triangles` _assimpimporter_2) :`Normals` (`AssimpImporterComponent.Normals` _assimpimporter_2) :`UV0` (`AssimpImporterComponent.UVs` _assimpimporter_2))
    (else
      (`KismetSystemLibrary.PrintString` (`KismetStringLibrary.Concat_StrStr` "Unable to load file : " _internalfilepath) true true (struct :`G` 0.66 :`B` 1.0 :`A` 1.0) 20.0))))

(fn `CreateNewMesh`
  (params (FilePath :type String))
  (bind _assimpimporter (`self.AssimpImporter`))
  (bind _generatedprocmeshcomp (`self.GeneratedProcMeshComp`))
  (bind _assimpimporter_2 (`self.AssimpImporter`))
  (bind _filepath (`self.FilePath`))
  ;[1 1 1] If reload destroy previous mesh
  (if (`KismetSystemLibrary.IsValid` _generatedprocmeshcomp)
    (`ActorComponent.K2_DestroyComponent` _generatedprocmeshcomp))
  ;[1 1 1] Load Mesh from file path or display error message
  (`self.SetFilePath` FilePath)
  (set `AssimpImporterComponent.InverseNormals` true _assimpimporter)
  (bind _returnvalue (`AssimpImporterComponent.Load3DModel` _assimpimporter _filepath))
  (if (not _returnvalue)
    (`KismetSystemLibrary.PrintString` (`KismetStringLibrary.Concat_StrStr` "Unable to load file : " _filepath) true true (struct :`G` 0.66 :`B` 1.0 :`A` 1.0) 20.0)
    (`self.SetFilePath` "")
    (`AssimpImporterComponent.Load3DModel` (`self.AssimpImporter`) (`self.FilePath`)))
  ;[1 1 1] Create procedural mesh and texture it
  (bind _returnvalue_2 (`AddComponent|ProceduralMeshComponent_0`))
  (bind _output_get (set `self.GeneratedProcMeshComp` _returnvalue_2))
  (`AssimpImporterComponent.SetMaterialToProceduralMeshComp` _assimpimporter_2 _output_get)
  (`ProceduralMeshComponent.CreateMeshSection` :`self` _returnvalue_2 :`Vertices` (`AssimpImporterComponent.Vertices` _assimpimporter_2) :`Triangles` (`AssimpImporterComponent.Triangles` _assimpimporter_2) :`Normals` (`AssimpImporterComponent.Normals` _assimpimporter_2) :`UV0` (`AssimpImporterComponent.UVs` _assimpimporter_2)))

(fn `SetFilePath`
  (params (Path :type String))
  ;[1 1 1] If given file path is not null set it to FilePath var otherwise use internal filepath
  (if (== (`KismetStringLibrary.Len` Path) 0)
    (set `self.FilePath` (`AssimpImporterComponent.InternalFilePath` (`self.AssimpImporter`)))
    (else
      (set `self.FilePath` Path))))

(fn `UserConstructionScript`
  (`self.CreateNewMesh` "D:\\Personal Dev Projects\\PortFolioApp\\Saved\\DiapoAssets\\Bird\\Beebird.obj"))