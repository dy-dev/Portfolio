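; BP_Import is an actor that loads a 3D model from a hardcoded local OBJ path and displays it as a procedural mesh.
; The construction script loads the file through AssimpImporter with inverted normals and builds a mesh section from its geometry, printing an error on failure.
; On BeginPlay, it applies a dynamic Bats_Mat instance to the mesh and feeds the importer's model texture into its texture parameter.
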(event `self.ReceiveBeginPlay`
  (`self.ChangeTexture`))

(event `self.ReceiveActorBeginOverlap`
  (params (OtherActor :type "Actor Object Reference")))

(event `self.ReceiveTick`
  (params (DeltaSeconds :type "Float (single-precision)")))

(fn `ChangeTexture`
  (bind _returnvalue (`KismetMaterialLibrary.CreateDynamicMaterialInstance` "/Game/Bats_Mat.Bats_Mat"))
  (bind _output_get (set `self.NewVar_0` _returnvalue))
  (`PrimitiveComponent.SetMaterial` (`self.NewVar_1`) 0 _output_get)
  (`MaterialInstanceDynamic.SetTextureParameterValue` (`self.NewVar_0`) "T2DParam" (`AssimpImporterComponent.ModelTexture` (`self.AssimpImporter`))))

(fn `CreateNewMesh`
  (params (FilePath :type String))
  (bind _filepath (`self.FilePath`))
  (bind _assimpimporter (`self.AssimpImporter`))
  (bind _assimpimporter_2 (`self.AssimpImporter`))
  (set `self.FilePath` FilePath)
  (set `AssimpImporterComponent.inverseNormals` true _assimpimporter)
  (set `AssimpImporterComponent.swapCoords` 0 _assimpimporter)
  (bind _returnvalue (`AssimpImporterComponent.Load` _assimpimporter _filepath))
  (if _returnvalue
    (bind _returnvalue_2 (`AddComponent|ProceduralMeshComponent_0`))
    (bind _output_get (set `self.NewVar_1` _returnvalue_2))
    (`ProceduralMeshComponent.CreateMeshSection` :`self` _output_get :`Vertices` (`AssimpImporterComponent.Vertices` _assimpimporter_2) :`Triangles` (`AssimpImporterComponent.Triangles` _assimpimporter_2) :`Normals` (`AssimpImporterComponent.Normals` _assimpimporter_2) :`UV0` (`AssimpImporterComponent.UVs` _assimpimporter_2))
    (else
      (`KismetSystemLibrary.PrintString` (`KismetStringLibrary.Concat_StrStr` "Unable to load file : " _filepath) true true (struct :`G` 0.66 :`B` 1.0 :`A` 1.0) 20.0))))

(fn `UserConstructionScript`
  (`self.CreateNewMesh` "D:\\Personal Dev Projects\\PortFolioApp\\Saved\\3dLoad\\Bats.obj"))